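; Obstacle actor placed along the road spline that shatters when a car hits it.
; The construction script takes the spline of the first RoadGenerator in the level and sets location and rotation from Offset (distance along, right, up) and Rotation, so placement follows the road.
; On the first overlap only, a Car is notified via OnHitObstacle and the destructible mesh takes heavy damage with an impulse along the car's forward vector.
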(event EventBeginPlay)

(event Collision|EventActorBeginOverlap
  (params (OtherActor :type Actor%20Object%20Reference))
  (if (not (Variables|Default|GetHasTriggered))
    (Variables|Default|SetHasTriggered true)
    (bind _ascar (Utilities|Casting|CastToCar OtherActor))
    (Default|OnHitObstacle _ascar)
    (Game|Damage|ApplyDamage (Variables|Default|GetDestructibleMesh) 1e+03 (Transformation|GetActorLocation) (Transformation|GetActorForwardVector OtherActor) 0.0)))

(event EventTick
  (params (DeltaSeconds :type Float%20%28single-precision%29)))

(fn ConstructionScript
  (bind _offset (Variables|Default|Getoffset))
  (Utilities|FlowControl|Sequence
    (:then_0
      ;[1 1 1] Find spline reference
      (bind _outactors (Actor|GetAllActorsOfClass "/Game/Blueprints/Track/RoadGenerator.RoadGenerator_C"))
      (if (> (Utilities|Array|Length _outactors) 0)
        (LocalVariables|SetSpline (Variables|/Game/Blueprints/Track/RoadGenerator.RoadGenerator_C|GetSpline (Utilities|Array|Get(acopy) _outactors)))))
    (:then_1
      ;[1 1 1] Assign position and rotation
      (Transformation|SetActorLocation (+ (.Location (Math|Transform|BreakTransform (Spline|GetTransformatDistanceAlongSpline (LocalVariables|GetSpline) (.x _offset) "World" false))) (+ (* (Class|SplineComponent|GetRightVectoratDistanceAlongSpline (LocalVariables|GetSpline) (.x _offset) "World") (.y _offset)) (* (Class|SplineComponent|GetUpVectoratDistanceAlongSpline (LocalVariables|GetSpline) (.x _offset) "World") (.z _offset)))) false false)
      (Transformation|SetActorRotation (Math|Rotator|CombineRotators (Variables|Default|GetRotation) (.Rotation (Math|Transform|BreakTransform (Spline|GetTransformatDistanceAlongSpline (LocalVariables|GetSpline) (.x _offset) "World" false))))))))