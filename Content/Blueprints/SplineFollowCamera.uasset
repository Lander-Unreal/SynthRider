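; Camera actor that trails the player car along the road spline, fetching both references on BeginPlay.
; Each tick it samples the spline at the car's distance, builds an offset target transform, and smoothly interpolates toward it.
; The spline's X scale doubles as a blend between portrait and landscape aspect ratio and FOV.
; A hack skips samples with zero rotation to work around bad spline data.
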(event EventBeginPlay
  (Utilities|FlowControl|Sequence
    (:then_0
      (Variables|State|SetTargetSpline (.RoadSpline (CallFunction|GetRoadSpline))))
    (:then_1
      (Variables|State|SetTargetCar (.PlayerCar (CallFunction|GetPlayerCar))))))

(event EventTick
  (params (DeltaSeconds :type Float%20%28single-precision%29))
  (bind _targetcar (Variables|State|GetTargetCar))
  (bind _targetspline (Variables|State|GetTargetSpline))
  (bind _camera (Variables|Default|GetCamera))
  (bind _carmovement (Variables|/Game/Blueprints/CarBlueprints/Car.Car_C|GetCarMovement _targetcar))
  (bind _distancealongspline (Variables|/Game/Blueprints/CarBlueprints/CarMovement.CarMovement_C|GetDistanceAlongSpline _carmovement))
  (bind _returnvalue (Spline|GetTransformatDistanceAlongSpline _targetspline _distancealongspline "World" true))
  (bind (_location _rotation _scale) (Math|Transform|BreakTransform _returnvalue))
  (Utilities|FlowControl|Sequence
    (:then_0
      ;[1 1 1] Calculate target
      (if (and (Utilities|IsValid (Variables|State|GetTargetSpline)) (Utilities|IsValid (Variables|State|GetTargetCar)))
        ;;[1 1 1] Hack to fix garbage spline data
        (if (Utilities|Enum|NotEqual(Enum) _rotation "0, 0, 0" 0.0)
          (Variables|State|SetTargetTransform (Math|Transform|MakeTransform (+ _location (Math|Vector|RotateVector (Variables|Stats|GetSplineOffset) _rotation)) _rotation "1.000000,1.000000,1.000000"))
          (Class|CameraComponent|SetAspectRatio _camera (Math|Float|MapRangeClamped (.x _scale) 0.0 1.0 (Variables|Stats|GetPortraitAspect) (Variables|Stats|GetLandscapeAspect)))
          (Camera|SetFieldOfView _camera (Math|Float|MapRangeClamped (.x _scale) 0.0 1.0 (Variables|Default|GetPortraitFOV) (Variables|Default|GetLandscapeFOV))))))
    (:then_1
      (Transformation|SetActorTransform (Class|KismetMathLibrary|TInterpto (Transformation|GetActorTransform) (Variables|State|GetTargetTransform) (Utilities|Time|GetWorldDeltaSeconds) (Variables|Stats|GetInterpSpeed))))))

(fn ConstructionScript
  (Class|CameraComponent|SetAspectRatio (Variables|Default|GetCamera) (Variables|State|GetTargetAspectRatio)))