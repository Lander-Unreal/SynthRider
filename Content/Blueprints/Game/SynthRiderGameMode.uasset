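; SynthRiderGameMode is the game mode that runs the start and end of a SynthRider stage.
; On BeginPlay it spawns a SplineFollowCamera as the view target, disables pawn input and initializes the HUD.
; When the HUD's ReadyGoFinished event fires, it re-enables input and records the start timestamp.
; GameOver marks the stage complete, plays the finish sound, disables input and triggers the HUD widget's LevelComplete.
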(event Custom|ReadyGoFinished
  (bind _returnvalue (Game|GetPlayerController 0))
  (Input|EnableInput (Pawn|GetControlledPawn _returnvalue) _returnvalue)
  (Variables|Default|SetGameStartTimestamp (Utilities|Time|GetGameTimeinSeconds)))

(event Custom|GameOver
  (bind _returnvalue (Game|GetPlayerController 0))
  (Variables|Default|SetStageComplete true)
  (Audio|PlaySound2D "/Game/Audio/sfx_finish.sfx_finish")
  (Input|DisableInput (Pawn|GetControlledPawn _returnvalue) 0)
  (bind _assynth_rider_hud (Utilities|Casting|CastToSynthRiderHUD (HUD|GetHUD _returnvalue)))
  (Default|LevelComplete (Variables|/Game/Blueprints/UI/SynthRiderHUD.SynthRiderHUD_C|GetHUDWidget _assynth_rider_hud)))

(event EventBeginPlay
  (bind _returnvalue (Game|GetPlayerController 0))
  (Utilities|FlowControl|Sequence
    (:then_0
      (bind _returnvalue_2 (Game|SpawnActorfromClass "/Game/Blueprints/SplineFollowCamera.SplineFollowCamera_C" (Math|Transform|MakeTransform "0, 0, 0" "0, 0, 0" "1,1,1") "AlwaysSpawn" 0 0))
      (Game|Player|SetViewTargetwithBlend (Game|GetPlayerController 0) _returnvalue_2 0.0 "VTBlend_Linear" 0.0 true))
    (:then_1
      (Input|DisableInput (Pawn|GetControlledPawn _returnvalue) _returnvalue)
      (bind _assynth_rider_hud (Utilities|Casting|CastToSynthRiderHUD (HUD|GetHUD _returnvalue)))
      (EventDispatchers|AssignEventReadyGoFinished _assynth_rider_hud (delegate Custom|ReadyGoFinished))
      (Default|Initialize _assynth_rider_hud))))

(fn ConstructionScript)