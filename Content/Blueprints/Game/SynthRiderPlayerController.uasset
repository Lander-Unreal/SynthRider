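; Player controller for SynthRider that handles global keys for restarting and quitting, plus time-control shortcuts.
; Once the game mode reports the stage complete, any key press plays a one-time sound, waits out its duration, then opens the title level.
; Escape quits the game, and three numpad keys set global time dilation to slow, normal or fast speed.
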(event Input|KeyboardEvents|NumPadFour
  (params (Key :type Key%20Structure :default "AnyKey"))
  ;[1 1 1] Numpad time dilation VCR
  (:Pressed
    (Utilities|Time|SetGlobalTimeDilation 0.25)))

(event Input|KeyboardEvents|NumPadFive
  (params (Key :type Key%20Structure :default "AnyKey"))
  ;[1 1 1] Numpad time dilation VCR
  (:Pressed
    (Utilities|Time|SetGlobalTimeDilation 1.0)))

(event Input|KeyboardEvents|AnyKey
  (params (Key :type Key%20Structure :default "AnyKey"))
  (bind _presssound (Variables|Default|GetPressSound))
  ;[1 1 1] Restart game
  (:Pressed
    (if (Variables|/Game/Blueprints/Game/SynthRiderGameMode.SynthRiderGameMode_C|GetStageComplete (.SynthRiderGameMode (CallFunction|GetSynthRiderGameMode)))
      (Utilities|FlowControl|DoOnce false
        (:Completed
          (Audio|PlaySound2D _presssound)
          (Utilities|FlowControl|Delay (Variables|/Script/Engine.SoundBase|GetDuration _presssound))
          (Game|OpenLevel(byName) "TitleLevel"))))))

(event Input|KeyboardEvents|NumPadSix
  (params (Key :type Key%20Structure :default "AnyKey"))
  ;[1 1 1] Numpad time dilation VCR
  (:Pressed
    (Utilities|Time|SetGlobalTimeDilation 4.0)))

(event Input|KeyboardEvents|Escape
  (params (Key :type Key%20Structure :default "AnyKey"))
  ;[1 1 1] Quit game binding
  (:Pressed
    (Game|QuitGame 0 "Quit")))

(fn ConstructionScript)