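; Blueprint function library for SynthRider that gives shortcut access to core gameplay objects: the player car, road generator, road spline and game mode.
; Each getter returns its object with a Success flag, casting player pawn 0 to Car and the current game mode to SynthRiderGameMode.
; The road generator is the first RoadGenerator found by an uncached GetAllActorsOfClass search, which the road spline getter also relies on.
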(fn GetRoadSpline
  (bind (_roadgenerator _success) (CallFunction|GetRoadGenerator))
  (if _success
    (return (Variables|/Game/Blueprints/Track/RoadGenerator.RoadGenerator_C|GetSpline _roadgenerator) true)
    (else
      (return 0 false))))

(fn GetPlayerCar
  (bind _ascar (Utilities|Casting|CastToCar (Game|Player|GetPlayerPawn 0))
    (:then
      (return _ascar true))
    (:CastFailed
      (return 0 false))))

(fn GetRoadGenerator
  (bind _outactors (Actor|GetAllActorsOfClass 0 "/Game/Blueprints/Track/RoadGenerator.RoadGenerator_C"))
  (if (> (Utilities|Array|Length _outactors) 0)
    (return (Utilities|Array|Get(acopy) _outactors) true)
    (else
      (return 0 false))))

(fn GetSynthRiderGameMode
  (bind _assynth_rider_game_mode (Utilities|Casting|CastToSynthRiderGameMode (Game|GetGameMode))
    (:then
      (return _assynth_rider_game_mode true))
    (:CastFailed
      (return 0 false))))