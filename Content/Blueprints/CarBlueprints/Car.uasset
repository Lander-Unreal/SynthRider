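; Player-driven car that follows a road spline, passing horizontal and vertical input to its CarMovement component.
; Each tick it line-traces under the four wheels, setting mesh rotation and height from averaged normals and impact points relative to the spline.
; It then sets mesh rotation to a steering yaw scaled by lateral and forward speed.
; Obstacle hits trigger CarMovement's collision response and timed invincibility with flashing visibility.
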(event EventTick
  (params (DeltaSeconds :type Float%20%28single-precision%29))
  (Utilities|FlowControl|Sequence
    (:then_0
      (CallFunction|ApplySurfaceRotation))
    (:then_1
      (CallFunction|ApplyTurnRotation))))

(event Input|AxisEvents|InputAxisHorizontal
  (params (AxisValue :type Float%20%28single-precision%29))
  (Default|AddInputVector (Variables|Default|GetCarMovement) (Math|Vector2D|MakeVector2D AxisValue 0.0)))

(event Input|AxisEvents|InputAxisVertical
  (params (AxisValue :type Float%20%28single-precision%29))
  (Default|AddInputVector (Variables|Default|GetCarMovement) (Math|Vector2D|MakeVector2D 0.0 AxisValue)))

(fn ConstructionScript
  (bind _frontleftwheel (Variables|Default|GetFrontLeftWheel))
  (bind _output_get (Variables|State|SetGroundOffset (.z (+ (Variables|/Script/Engine.SceneComponent|GetRelativeLocation _frontleftwheel) (Math|Vector|MakeVector 0.0 0.0 (* (.z (.boxextent (StaticMesh|GetBounds (Variables|/Script/Engine.StaticMeshComponent|GetStaticMesh _frontleftwheel)))) 0.5))))))
  (Transformation|AddRelativeLocation (Variables|Default|GetStaticMesh) (Math|Vector|MakeVector 0.0 0.0 _output_get) false false))

(fn ApplyTurnRotation
  (bind _carmovement (Variables|Default|GetCarMovement))
  (Transformation|SetRelativeRotation (Variables|Default|GetStaticMesh) (Math|Rotator|MakeRotator 0.0 0.0 (* (* (/ (.x (Variables|/Game/Blueprints/CarBlueprints/CarMovement.CarMovement_C|GetOffsetVelocity _carmovement)) (.x (Variables|/Game/Blueprints/CarBlueprints/CarMovement.CarMovement_C|GetMaxOffsetVelocity _carmovement))) (/ (Variables|/Game/Blueprints/CarBlueprints/CarMovement.CarMovement_C|GetDistanceVelocity _carmovement) (Variables|/Game/Blueprints/CarBlueprints/CarMovement.CarMovement_C|GetMaxDistanceVelocity _carmovement))) (Variables|Stats|GetTurnAngle))) false false))

(fn RaycastfromWheel
  (params (WheelLocation :type Vector))
  (bind _returnvalue (Transformation|GetActorUpVector))
  (bind _returnvalue_2 (* _returnvalue 5e+01))
  (bind (_outhit _returnvalue_3) (Collision|LineTraceForObjects (+ WheelLocation _returnvalue_2) (- WheelLocation _returnvalue_2) (Utilities|Array|MakeArray "ObjectTypeQuery1") true 0 "None"))
  (if _returnvalue_3
    (return (.ImpactPoint (Collision|BreakHitResult _outhit)) (.ImpactNormal (Collision|BreakHitResult _outhit)) true)
    (else
      (return "0, 0, 0" "0, 0, 0" false))))

(fn ApplySurfaceRotation
  (bind _wheelmeshes (LocalVariables|GetWheelMeshes))
  (Utilities|Array|AddUnique _wheelmeshes (Variables|Default|GetFrontLeftWheel))
  (Utilities|Array|AddUnique _wheelmeshes (Variables|Default|GetFrontRightWheel))
  (Utilities|Array|AddUnique _wheelmeshes (Variables|Default|GetBackRightWheel))
  (Utilities|Array|AddUnique _wheelmeshes (Variables|Default|GetBackLeftWheel))
  (for _array_element _wheelmeshes
    (bind (_impactpoint _impactnormal _hit) (CallFunction|RaycastfromWheel (+ (Transformation|GetActorLocation) (Math|Transform|TransformDirection (Transformation|GetActorTransform) (Variables|/Script/Engine.SceneComponent|GetRelativeLocation _array_element)))))
    (if _hit
      (Utilities|Array|Add (LocalVariables|GetSurfaceNormals) _impactnormal)
      (Utilities|Array|Add (LocalVariables|GetImpactPoints) _impactpoint)))
  (Utilities|FlowControl|Sequence
    (:then_0
      (Transformation|SetRelativeRotation (Variables|Default|GetStaticMesh) (Math|Rotator|MakeRotfromZX (Math|Vector|Normalize (Math|Vector|GetVectorArrayAverage (LocalVariables|GetSurfaceNormals))) (Transformation|GetActorForwardVector)) false false))
    (:then_1
      (Transformation|SetRelativeLocation (Variables|Default|GetStaticMesh) (Math|Vector|MakeVector 0.0 0.0 (+ (.z (Math|Vector|UnrotateVector (- (Math|Vector|GetVectorArrayAverage (LocalVariables|GetImpactPoints)) (Spline|GetLocationatDistanceAlongSpline (.RoadSpline (CallFunction|GetRoadSpline)) (Variables|/Game/Blueprints/CarBlueprints/CarMovement.CarMovement_C|GetDistanceAlongSpline (Variables|Default|GetCarMovement)) "World")) (Transformation|GetActorRotation))) (Variables|State|GetGroundOffset))) false true))))

(fn OnHitObstacle
  (if (not (Variables|State|Invincibility|GetIsInvincible))
    (Default|HandleObstacleCollision (Variables|Default|GetCarMovement))
    (Variables|State|Invincibility|SetIsInvincible true)
    (Utilities|Time|SetTimerbyEvent (EventDispatchers|CreateEvent :!event DeactivateInvincibility) (Variables|Stats|Invincibility|GetInvincibilityDuration))
    (bind _returnvalue (Utilities|Time|SetTimerbyEvent (EventDispatchers|CreateEvent :!event ToggleInvinicibilityFlash) (Variables|Stats|Invincibility|GetInvincibilityFlashDuration) true))
    (Variables|State|Invincibility|SetInvincibilityFlashTimerHandle _returnvalue)))

(fn DeactivateInvincibility
  (Variables|State|Invincibility|SetIsInvincible false)
  (Utilities|Time|ClearandInvalidateTimerbyHandle (Variables|State|Invincibility|GetInvincibilityFlashTimerHandle))
  (Rendering|SetVisibility (Variables|Default|GetStaticMesh) true true))

(fn ToggleInvinicibilityFlash
  (bind _staticmesh (Variables|Default|GetStaticMesh))
  (Rendering|SetVisibility _staticmesh (not (Variables|/Script/Engine.SceneComponent|GetbVisible _staticmesh)) true))