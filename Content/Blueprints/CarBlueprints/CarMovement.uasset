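; Car movement component that drives its owner along the road spline as a distance plus a lateral offset, in place of physics.
; Each tick turns accumulated input into speed and steering velocity, with deceleration, clamping to limits and road width, and speed-curved handling.
; Countersteer samples the spline ahead to push the car outward on bends.
; It also slows on obstacle collisions and calls GameOver at the spline's end.
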(event EventTick
  (params (DeltaSeconds :type Float%20%28single-precision%29))
  (Utilities|FlowControl|Sequence
    (:then_0
      ;[1 1 1] Lateral Movement
      (CallFunction|ApplySteerInput))
    (:then_1
      (CallFunction|ApplySteerDeceleration))
    (:then_2
      (CallFunction|ApplyCountersteer))
    (:then_3
      (CallFunction|ApplyOffsetVelocity))
    (:then_4
      (CallFunction|ClampOffset))
    (:then_5
      ;[1 1 1] Forward Movement
      (CallFunction|ApplyAccelerationInput))
    (:then_6
      (CallFunction|ApplyDistanceDeceleration))
    (:then_7
      (CallFunction|ApplyDistanceVelocity))
    (:then_8
      (CallFunction|ClampVelocity))
    (:then_9
      (CallFunction|ApplySplineTransform))
    (:then_10
      ;[1 1 1] Consume input vector
      (Variables|State|SetInputVector ""))
    (:then_11
      (CallFunction|CheckFinished))))

(fn AddInputVector
  (params (Vector :type Vector%202D%20Structure))
  (Variables|State|SetInputVector (+ (Variables|State|GetInputVector) Vector)))

(fn ApplySteerInput
  ;[1 1 1] Process horizontal input vector
  (Variables|State|SetOffsetVelocity (+ (Variables|State|GetOffsetVelocity) (Math|Vector2D|MakeVector2D (* (* (* (.x (Variables|State|GetInputVector)) (Variables|Stats|GetSteerIntensity)) (Math|Curves|GetFloatValue (Variables|Default|GetHandlingCurve) (Utilities|GetDistanceVelocityScalar))) (Utilities|Time|GetWorldDeltaSeconds)) 0.0))))

(fn ApplySteerDeceleration
  ;[1 1 1] Decelerate offset velocity
  (if (== (.x (Variables|State|GetInputVector)) 0.0)
    (bind _output_get (LocalVariables|SetVelocitySign (Math|Float|Sign(Float) (.X (Math|Vector2D|BreakVector2D (Variables|State|GetOffsetVelocity))))))
    (Variables|State|SetOffsetVelocity (Math|Vector2D|MakeVector2D (* (Math|Float|Max(Float) (- (Math|Float|Absolute(Float) (.X (Math|Vector2D|BreakVector2D (Variables|State|GetOffsetVelocity)))) (* (Utilities|Time|GetWorldDeltaSeconds) (Variables|Stats|GetOffsetDeceleration))) 0.0) _output_get) (.Y (Math|Vector2D|BreakVector2D (Variables|State|GetOffsetVelocity)))))))

(fn ApplyAccelerationInput
  ;[1 1 1] Process vertical input vector
  (Variables|State|SetDistanceVelocity (+ (* (* (.y (Variables|State|GetInputVector)) (Variables|Stats|GetAcceleration)) (Utilities|Time|GetWorldDeltaSeconds)) (Variables|State|GetDistanceVelocity))))

(fn ApplyOffsetVelocity
  ;[1 1 1] Apply offset velocity
  (Variables|State|SetSplineOffset (+ (Variables|State|GetSplineOffset) (* (Variables|State|GetOffsetVelocity) (Utilities|Time|GetWorldDeltaSeconds)))))

(fn ApplyDistanceVelocity
  ;[1 1 1] Apply distance velocity
  (Variables|State|SetDistanceAlongSpline (+ (Variables|State|GetDistanceAlongSpline) (* (Variables|State|GetDistanceVelocity) (Utilities|Time|GetWorldDeltaSeconds)))))

(fn ApplySplineTransform
  (bind _roadspline (CallFunction|GetRoadSpline))
  (bind _splineoffset (Variables|State|GetSplineOffset))
  (bind _distancealongspline (Variables|State|GetDistanceAlongSpline))
  (bind _returnvalue (Spline|GetTransformatDistanceAlongSpline _roadspline _distancealongspline "World" false))
  (bind (_location _rotation) (Math|Transform|BreakTransform _returnvalue))
  ;[1 1 1] Position owner along spline acording to distance and offset
  (Transformation|SetActorLocationAndRotation (Components|GetOwner) (+ (Math|Transform|TransformDirection _returnvalue (Math|Vector|MakeVector 0.0 (.x _splineoffset) (.y _splineoffset))) _location) _rotation))

(fn ApplyCountersteer
  (bind _roadspline (CallFunction|GetRoadSpline))
  (bind _distancealongspline (Variables|State|GetDistanceAlongSpline))
  (bind _returnvalue (Spline|GetDirectionatDistanceAlongSpline _roadspline _distancealongspline "World"))
  (bind _maskedvector (Utilities|XYMaskVector _returnvalue))
  (bind _returnvalue_2 (Math|Vector|Normalize _maskedvector))
  (for _index (range 0 (- (LocalVariables|GetSubdivisions) 1))
    (LocalVariables|SetSplineAngleAccumulator (+ (LocalVariables|GetSplineAngleAccumulator) (* (Math|Trig|Acos(Degrees) (Math|Vector|DotProduct _returnvalue_2 (Math|Vector|Normalize (- (Utilities|XYMaskVector (Spline|GetLocationatDistanceAlongSpline _roadspline (+ _distancealongspline (* _index (LocalVariables|GetSubdivisionLength))) "World")) (Utilities|XYMaskVector (Spline|GetLocationatDistanceAlongSpline _roadspline _distancealongspline "World")))))) (Math|Float|Sign(Float) (Math|Vector|DotProduct (Math|Vector|CrossProduct _returnvalue_2 (Math|Vector|Normalize (- (Utilities|XYMaskVector (Spline|GetLocationatDistanceAlongSpline _roadspline (+ _distancealongspline (* _index (LocalVariables|GetSubdivisionLength))) "World")) (Utilities|XYMaskVector (Spline|GetLocationatDistanceAlongSpline _roadspline _distancealongspline "World"))))) "0, 0,1.000000"))))))
  ;[1 1 1] Apply countersteer velocity
  (Variables|State|SetOffsetVelocity (+ (Variables|State|GetOffsetVelocity) (Math|Vector2D|MakeVector2D (* (* (* (* (LocalVariables|GetSplineAngleAccumulator) -1.0) (Utilities|GetDistanceVelocityScalar)) (Variables|Stats|GetCountersteerIntensity)) (Utilities|Time|GetWorldDeltaSeconds)) 0.0))))

(fn ClampVelocity
  (bind _maxoffsetvelocity (Variables|Stats|GetMaxOffsetVelocity))
  (Utilities|FlowControl|Sequence
    (:then_0
      ;[1 1 1] Clamp distance velocity
      (Variables|State|SetDistanceVelocity (Math|Float|Clamp(Float) (Variables|State|GetDistanceVelocity) 0.0 (Variables|Stats|GetMaxDistanceVelocity))))
    (:then_1
      ;[1 1 1] Clamp offset velocity
      (Variables|State|SetOffsetVelocity (Math|Vector2D|MakeVector2D (Math|Float|Clamp(Float) (.X (Math|Vector2D|BreakVector2D (Variables|State|GetOffsetVelocity))) (* (.x _maxoffsetvelocity) -1.0) (.x _maxoffsetvelocity)) (Math|Float|Clamp(Float) (.Y (Math|Vector2D|BreakVector2D (Variables|State|GetOffsetVelocity))) (* -1.0 (.y _maxoffsetvelocity)) (.y _maxoffsetvelocity)))))))

(fn ApplyDistanceDeceleration
  ;[1 1 1] Decelerate distance velocity
  (if (== (.y (Variables|State|GetInputVector)) 0.0)
    (Variables|State|SetDistanceVelocity (Math|Float|Max(Float) (- (Variables|State|GetDistanceVelocity) (* (Variables|Stats|GetDistanceDeceleration) (Utilities|Time|GetWorldDeltaSeconds))) 0.0))))

(fn HandleObstacleCollision
  (Variables|State|SetDistanceVelocity (* (Variables|State|GetDistanceVelocity) (Variables|Stats|GetCollisionVelocityMultiplier))))

(fn ClampOffset
  (bind _playercar (CallFunction|GetPlayerCar))
  (bind _roadspline (CallFunction|GetRoadSpline))
  (bind _roadgenerator (CallFunction|GetRoadGenerator))
  (bind _distancealongspline (Variables|State|GetDistanceAlongSpline))
  (bind _returnvalue (Class|SplineComponent|GetScaleatDistanceAlongSpline _roadspline _distancealongspline))
  (bind _staticmesh (Variables|/Game/Blueprints/CarBlueprints/Car.Car_C|GetStaticMesh _playercar))
  (bind _splinemesh (Variables|/Game/Blueprints/Track/RoadGenerator.RoadGenerator_C|GetSplineMesh _roadgenerator))
  (bind _returnvalue_2 (StaticMesh|GetBounds _splinemesh))
  (bind _staticmesh_2 (Variables|/Script/Engine.StaticMeshComponent|GetStaticMesh _staticmesh))
  (bind _returnvalue_3 (StaticMesh|GetBounds _staticmesh_2))
  (bind _returnvalue_4 (* (.y _returnvalue) (.y (.boxextent _returnvalue_2))))
  (bind _returnvalue_5 (- _returnvalue_4 (.y (.boxextent _returnvalue_3))))
  (Variables|State|SetSplineOffset (Math|Vector2D|MakeVector2D (Math|Float|Clamp(Float) (.X (Math|Vector2D|BreakVector2D (Variables|State|GetSplineOffset))) (* _returnvalue_5 -1.0) _returnvalue_5) (.Y (Math|Vector2D|BreakVector2D (Variables|State|GetSplineOffset))))))

(fn CheckFinished
  (bind _synthridergamemode (CallFunction|GetSynthRiderGameMode))
  (if (and (not (Variables|/Game/Blueprints/Game/SynthRiderGameMode.SynthRiderGameMode_C|GetStageComplete _synthridergamemode)) (>= (Utilities|GetDistanceAlongSplineScalar) 1.0))
    (Default|GameOver _synthridergamemode)))