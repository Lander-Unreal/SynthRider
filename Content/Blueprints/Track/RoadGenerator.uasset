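; Road generator actor that builds a track from a spline in the construction script.
; It adds one spline mesh per segment between neighboring points, plus a closing segment when the spline is set as a closed loop.
; Each segment gets the configured mesh, material and BlockAll collision.
; Location, tangent, roll and Y/Z scale come from its end points, so banking and width are shaped on the spline itself.
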(fn ConstructionScript
  (bind _spline (Variables|Default|GetSpline))
  (bind _returnvalue (Spline|GetNumberOfSplinePoints _spline))
  (Spline|SetClosedLoop (Variables|Default|GetSpline) (Variables|Default|GetIsClosedLoop) true)
  (for _index (range 0 (- _returnvalue 2))
    (Utilities|CreateSplineMeshforIndices _index (+ _index 1)))
  (if (Class|SplineComponent|IsClosedLoop (Variables|Default|GetSpline))
    (Utilities|CreateSplineMeshforIndices (- _returnvalue 1) 0)))